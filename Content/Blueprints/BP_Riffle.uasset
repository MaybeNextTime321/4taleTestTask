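; BP_Riffle is a hitscan rifle owned by the third-person character.
; Shoot calls ShootOnServer, which casts the owner and traces on the Visibility channel from the muzzle socket along the follow camera's forward vector.
; The hit actor takes fixed damage, and each trace leaves a persistent debug line.
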(event Custom|ShootOnServer
  (bind _skeletalmesh (Variables|Default|GetSkeletalMesh))
  (bind _returnvalue (Transformation|GetSocketLocation _skeletalmesh "MuzzleFlashSocket"))
  (bind _asbp_third_person_character (Utilities|Casting|CastToBP_ThirdPersonCharacter (Components|GetOwner)))
  (bind _outhit (Collision|LineTraceByChannel _returnvalue (+ _returnvalue (* (Math|Vector|GetForwardVector (Variables|/Script/TestTask4Tale.TestTask4TaleCharacter|GetFollowCamera _asbp_third_person_character)) 4000)) "TraceTypeQuery1" false 0 "Persistent"))
  (Game|Damage|ApplyDamage (.hitactor _outhit) 25.0 0 0))

(event EventBeginPlay)

(event Collision|EventActorBeginOverlap
  (params (OtherActor :type Actor%20Object%20Reference)))

(event EventTick
  (params (DeltaSeconds :type Float%20%28single-precision%29)))

(event EventShoot
  (CallFunction|ShootonServer))

(fn ConstructionScript)